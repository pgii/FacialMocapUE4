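; UDP server controller that receives facial capture data over the network and passes it to the facial mocap controller.
; On BeginPlay it listens on a UDP socket and binds a handler for incoming bytes, closing the socket on EndPlay.
; The handler parses the bytes as JSON and, for facial data messages, converts mouth, brow and blink fields from strings to floats and sends them to the first FacialMocapController found in the level.
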(event Custom|UDPReceivedEvent
  (params (Bytes :type Array%20of%20Bytes))
  (bind _returnvalue (Class|UDPComponent|StringfromBinaryArray (Variables|Default|GetUDP) Bytes))
  (bind _returnvalue_2 (Class|SIOJsonValue|AsObject (Class|SIOJsonValue|ValuefromJsonString _returnvalue)))
  (if (Utilities|Enum|Equal(Enum) (Class|SIOJsonObject|GetStringField _returnvalue_2 "type") "facialData")
    (bind _outactors (Actor|GetAllActorsOfClass "/Game/Blueprints/FacialMocapController.FacialMocapController_C"))
    (Default|FacialDataReceive (Utilities|Array|Get(acopy) _outactors) (Math|Conversions|ToFloat(Integer) (Class|SIOJsonObject|GetStringField _returnvalue_2 "mouthOpen")) (Math|Conversions|ToFloat(Integer) (Class|SIOJsonObject|GetStringField _returnvalue_2 "mouthTight")) (Math|Conversions|ToFloat(Integer) (Class|SIOJsonObject|GetStringField _returnvalue_2 "mouthSmileLeft")) (Math|Conversions|ToFloat(Integer) (Class|SIOJsonObject|GetStringField _returnvalue_2 "mouthSmileRight")) (Math|Conversions|ToFloat(Integer) (Class|SIOJsonObject|GetStringField _returnvalue_2 "mouthNarrowLeft")) (Math|Conversions|ToFloat(Integer) (Class|SIOJsonObject|GetStringField _returnvalue_2 "mouthNarrowRight")) (Math|Conversions|ToFloat(Integer) (Class|SIOJsonObject|GetStringField _returnvalue_2 "browUpLeft")) (Math|Conversions|ToFloat(Integer) (Class|SIOJsonObject|GetStringField _returnvalue_2 "browUpRight")) (Math|Conversions|ToFloat(Integer) (Class|SIOJsonObject|GetStringField _returnvalue_2 "eyeBlinkLeft")) (Math|Conversions|ToFloat(Integer) (Class|SIOJsonObject|GetStringField _returnvalue_2 "eyeBlinkRight")))))

(event EventBeginPlay
  (bind _udp (Variables|Default|GetUDP))
  (Class|UDPComponent|StartReceiveSocketListening _udp 7755)
  (EventDispatchers|BindEventtoOnReceivedBytes _udp (delegate Custom|UDPReceivedEvent)))

(event EventEndPlay
  (params (EndPlayReason :type EEndPlayReason%20Enum :default "Destroyed"))
  (Class|UDPComponent|CloseReceiveSocket (Variables|Default|GetUDP)))

(fn ConstructionScript)