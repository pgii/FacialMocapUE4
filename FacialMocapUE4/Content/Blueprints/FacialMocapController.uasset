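; Facial mocap controller that drives Genesis 8 Female morph targets for mouth, brows and eye blinks on a skeletal mesh.
; FacialDataReceive takes a set of expression values and fans them out through a sequence to one setter event per morph.
; Each setter smooths with FInterpTo using shared delta time and speed variables, interpolating from the incoming value toward the existing weight, the reverse of the usual argument order.
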(event Custom|FacialDataReceive
  (params (mouthOpen :type Float%20%28single-precision%29) (mouthTight :type Float%20%28single-precision%29) (mouthSmileLeft :type Float%20%28single-precision%29) (mouthSmileRight :type Float%20%28single-precision%29) (mouthNarrowLeft :type Float%20%28single-precision%29) (mouthNarrowRight :type Float%20%28single-precision%29) (browUpLeft :type Float%20%28single-precision%29) (browUpRight :type Float%20%28single-precision%29) (eyeBlinkLeft :type Float%20%28single-precision%29) (eyeBlinkRight :type Float%20%28single-precision%29))
  (Utilities|FlowControl|Sequence
    (:then_0
      (CallFunction|SetMouthOpen mouthOpen))
    (:then_1
      (CallFunction|SetMouthTight mouthTight))
    (:then_2
      (CallFunction|SetMouthSmileLeft mouthSmileLeft))
    (:then_3
      (CallFunction|SetMouthSmileRight mouthSmileRight))
    (:then_4
      (CallFunction|SetMouthNarrowLeft mouthNarrowLeft))
    (:then_5
      (CallFunction|SetMouthNarrowRight mouthNarrowRight))
    (:then_6
      (CallFunction|SetBrowUpLeft browUpLeft))
    (:then_7
      (CallFunction|SetBrowUpRight browUpRight))
    (:then_8
      (CallFunction|SetEyeBlinkLeft eyeBlinkLeft))
    (:then_9
      (CallFunction|SetEyeBlinkRight eyeBlinkRight))))

(event Custom|SetEyeBlinkRight
  (params (value :type Float%20%28single-precision%29))
  (bind _skeletalmesh (Variables|Default|GetSkeletalMesh))
  (bind _skeletalmeshcomponent (Variables|/Script/Engine.SkeletalMeshActor|GetSkeletalMeshComponent _skeletalmesh))
  (Components|SkeletalMesh|SetMorphTarget _skeletalmeshcomponent "Genesis8Female__eCTRLEyesClosedR" (Math|Interpolation|FInterpTo value (Class|SkeletalMeshComponent|GetMorphTarget _skeletalmeshcomponent "Genesis8Female__eCTRLEyesClosedR") (Variables|Default|GetSmoothDeltaTime) (Variables|Default|GetSmoothInterpSpeed)) true))

(event Custom|SetBrowUpLeft
  (params (value :type Float%20%28single-precision%29))
  (bind _skeletalmesh (Variables|Default|GetSkeletalMesh))
  (bind _skeletalmeshcomponent (Variables|/Script/Engine.SkeletalMeshActor|GetSkeletalMeshComponent _skeletalmesh))
  (Components|SkeletalMesh|SetMorphTarget _skeletalmeshcomponent "Genesis8Female__eCTRLBrowUp-DownL" (Math|Interpolation|FInterpTo value (Class|SkeletalMeshComponent|GetMorphTarget _skeletalmeshcomponent "Genesis8Female__eCTRLBrowUp-DownL") (Variables|Default|GetSmoothDeltaTime) (Variables|Default|GetSmoothInterpSpeed)) true))

(event Custom|SetBrowUpRight
  (params (value :type Float%20%28single-precision%29))
  (bind _skeletalmesh (Variables|Default|GetSkeletalMesh))
  (bind _skeletalmeshcomponent (Variables|/Script/Engine.SkeletalMeshActor|GetSkeletalMeshComponent _skeletalmesh))
  (Components|SkeletalMesh|SetMorphTarget _skeletalmeshcomponent "Genesis8Female__eCTRLBrowUp-DownR" (Math|Interpolation|FInterpTo value (Class|SkeletalMeshComponent|GetMorphTarget _skeletalmeshcomponent "Genesis8Female__eCTRLBrowUp-DownR") (Variables|Default|GetSmoothDeltaTime) (Variables|Default|GetSmoothInterpSpeed)) true))

(event Custom|SetMouthOpen
  (params (value :type Float%20%28single-precision%29))
  (bind _skeletalmesh (Variables|Default|GetSkeletalMesh))
  (bind _skeletalmeshcomponent (Variables|/Script/Engine.SkeletalMeshActor|GetSkeletalMeshComponent _skeletalmesh))
  (Components|SkeletalMesh|SetMorphTarget _skeletalmeshcomponent "Genesis8Female__eCTRLMouthOpen" (Math|Interpolation|FInterpTo value (Class|SkeletalMeshComponent|GetMorphTarget _skeletalmeshcomponent "Genesis8Female__eCTRLMouthOpen") (Variables|Default|GetSmoothDeltaTime) (Variables|Default|GetSmoothInterpSpeed)) true))

(event Custom|SetMouthTight
  (params (value :type Float%20%28single-precision%29))
  (bind _skeletalmesh (Variables|Default|GetSkeletalMesh))
  (bind _skeletalmeshcomponent (Variables|/Script/Engine.SkeletalMeshActor|GetSkeletalMeshComponent _skeletalmesh))
  (Components|SkeletalMesh|SetMorphTarget _skeletalmeshcomponent "Genesis8Female__40_Mouth_Lips_Tight" (Math|Interpolation|FInterpTo value (Class|SkeletalMeshComponent|GetMorphTarget _skeletalmeshcomponent "Genesis8Female__40_Mouth_Lips_Tight") (Variables|Default|GetSmoothDeltaTime) (Variables|Default|GetSmoothInterpSpeed)) true))

(event Custom|SetMouthSmileLeft
  (params (value :type Float%20%28single-precision%29))
  (bind _skeletalmesh (Variables|Default|GetSkeletalMesh))
  (bind _skeletalmeshcomponent (Variables|/Script/Engine.SkeletalMeshActor|GetSkeletalMeshComponent _skeletalmesh))
  (Components|SkeletalMesh|SetMorphTarget _skeletalmeshcomponent "Genesis8Female__27_Mouth_Smile_L" (Math|Interpolation|FInterpTo value (Class|SkeletalMeshComponent|GetMorphTarget _skeletalmeshcomponent "Genesis8Female__27_Mouth_Smile_L") (Variables|Default|GetSmoothDeltaTime) (Variables|Default|GetSmoothInterpSpeed)) true))

(event Custom|SetEyeBlinkLeft
  (params (value :type Float%20%28single-precision%29))
  (bind _skeletalmesh (Variables|Default|GetSkeletalMesh))
  (bind _skeletalmeshcomponent (Variables|/Script/Engine.SkeletalMeshActor|GetSkeletalMeshComponent _skeletalmesh))
  (Components|SkeletalMesh|SetMorphTarget _skeletalmeshcomponent "Genesis8Female__eCTRLEyesClosedL" (Math|Interpolation|FInterpTo value (Class|SkeletalMeshComponent|GetMorphTarget _skeletalmeshcomponent "Genesis8Female__eCTRLEyesClosedL") (Variables|Default|GetSmoothDeltaTime) (Variables|Default|GetSmoothInterpSpeed)) true))

(event Custom|SetMouthSmileRight
  (params (value :type Float%20%28single-precision%29))
  (bind _skeletalmesh (Variables|Default|GetSkeletalMesh))
  (bind _skeletalmeshcomponent (Variables|/Script/Engine.SkeletalMeshActor|GetSkeletalMeshComponent _skeletalmesh))
  (Components|SkeletalMesh|SetMorphTarget _skeletalmeshcomponent "Genesis8Female__28_Mouth_Smile_R" (Math|Interpolation|FInterpTo value (Class|SkeletalMeshComponent|GetMorphTarget _skeletalmeshcomponent "Genesis8Female__28_Mouth_Smile_R") (Variables|Default|GetSmoothDeltaTime) (Variables|Default|GetSmoothInterpSpeed)) true))

(event Custom|SetMouthNarrowLeft
  (params (value :type Float%20%28single-precision%29))
  (bind _skeletalmesh (Variables|Default|GetSkeletalMesh))
  (bind _skeletalmeshcomponent (Variables|/Script/Engine.SkeletalMeshActor|GetSkeletalMeshComponent _skeletalmesh))
  (Components|SkeletalMesh|SetMorphTarget _skeletalmeshcomponent "Genesis8Female__eCTRLMouthNarrowL" (Math|Interpolation|FInterpTo value (Class|SkeletalMeshComponent|GetMorphTarget _skeletalmeshcomponent "Genesis8Female__eCTRLMouthNarrowL") (Variables|Default|GetSmoothDeltaTime) (Variables|Default|GetSmoothInterpSpeed)) true))

(event Custom|SetMouthNarrowRight
  (params (value :type Float%20%28single-precision%29))
  (bind _skeletalmesh (Variables|Default|GetSkeletalMesh))
  (bind _skeletalmeshcomponent (Variables|/Script/Engine.SkeletalMeshActor|GetSkeletalMeshComponent _skeletalmesh))
  (Components|SkeletalMesh|SetMorphTarget _skeletalmeshcomponent "Genesis8Female__eCTRLMouthNarrowR" (Math|Interpolation|FInterpTo value (Class|SkeletalMeshComponent|GetMorphTarget _skeletalmeshcomponent "Genesis8Female__eCTRLMouthNarrowR") (Variables|Default|GetSmoothDeltaTime) (Variables|Default|GetSmoothInterpSpeed)) true))

(fn ConstructionScript)